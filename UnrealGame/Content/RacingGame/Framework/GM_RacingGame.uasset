(event Custom|Game%20Start
  (Development|PrintString "Game Started")
  (Utilities|Time|SetTimerbyEvent (delegate Custom|Lose_OutOfTime) (Variables|Default|GetStartTimerDuration)))

(event Custom|Game%20End
  (Development|PrintString (Utilities|String|SelectString "You won" "You lost" true)))

(event Custom|Start%20Countdown
  (Development|PrintString "Countdown has started")
  (Utilities|FlowControl|Delay (Variables|Default|GetStartCountdownDuration))
  (CallFunction|GameStart))

(event Custom|Lose_OutOfTime
  (CallFunction|GameEnd))

(event EventBeginPlay
  (CallFunction|StartCountdown))

(event EventTick
  (params (DeltaSeconds :type Float%20%28single-precision%29)))

(fn ConstructionScript)